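; BP_FrontController is the front-end controller that brings up the opening press-any-key screen.
; When the loading screen deactivates, it creates the primary layout widget, registers it with the Front UI subsystem and pushes that screen onto the front widget stack by gameplay tag as a soft class.
; It then registers the character input mapping context with the Enhanced Input user settings.
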(event `self.ReceivePossess`
  (params (PossessedPawn :type "Pawn Object Reference")))

(event `LoadingScreenInterface.OnLoadingScreenDeactivated`
  (`|ExecutionSequence`
    (:`then_0`
      (bind _returnvalue (`|CreateWidget` "/Game/UI/FrontWidgets/WBP_CUW_PrimaryLayout.WBP_CUW_PrimaryLayout_C" self))
      (`UserWidget.AddToViewport` _returnvalue 0)
      (`FrontUISubsystem.RegisterCreatedPrimaryLayout` (subsystem `FrontUISubsystem`) _returnvalue)
      (`AsyncActionPushSoftWidget.PushSoftWidget` self (`FrontFunctionLibrary.GetFrontSoftWidgetClassByTag` (struct :`TagName` "Front.Widget.PressAnyKeyScreen")) (struct :`TagName` "Front.WidgetStack.Front")))
    (:`then_1`
      (`EnhancedInputUserSettings.RegisterInputMappingContext` (`EnhancedInputSubsystemInterface.GetUserSettings` (subsystem `EnhancedInputLocalPlayerSubsystem`)) "/Game/Inputs/IMC_CharacterInputMapping.IMC_CharacterInputMapping"))))

(fn `UserConstructionScript`)